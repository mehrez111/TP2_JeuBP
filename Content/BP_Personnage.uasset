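; BP_Personnage is a player character driven by Enhanced Input that can move, look, jump and spawn water cubes.
; Movement follows the actor's forward and right vectors, while look inputs feed controller pitch and yaw.
; The throw action spawns a BP_CubeEau at an offset rotated by the actor's rotation, with no launch force applied here, and prints a confirmation message.
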(event `EnhancedInput|/Game/Inputs/IA_BougeAvantArriere`
  (params (ActionValue :type "Float (double-precision)") (ElapsedSeconds :type "Float (double-precision)") (TriggeredSeconds :type "Float (double-precision)") (InputAction :type "InputAction Object Reference" :default "/Game/Inputs/IA_BougeAvantArriere.IA_BougeAvantArriere"))
  ;[1 1 1] Bouger avant / arriere
  (:`Triggered`
    (`self.AddMovementInput` (`KismetMathLibrary.GetForwardVector` (`self.K2_GetActorRotation`)) ActionValue)))

(event `EnhancedInput|/Game/Inputs/IA_BougerGaucheDroite`
  (params (ActionValue :type "Float (double-precision)") (ElapsedSeconds :type "Float (double-precision)") (TriggeredSeconds :type "Float (double-precision)") (InputAction :type "InputAction Object Reference" :default "/Game/Inputs/IA_BougerGaucheDroite.IA_BougerGaucheDroite"))
  ;[1 1 1] Bouger Gauche / Droite
  (:`Triggered`
    (`self.AddMovementInput` (`KismetMathLibrary.GetRightVector` (`self.K2_GetActorRotation`)) ActionValue)))

(event `EnhancedInput|/Game/Inputs/IA_Sauter`
  (params (ActionValue :type Boolean) (ElapsedSeconds :type "Float (double-precision)") (TriggeredSeconds :type "Float (double-precision)") (InputAction :type "InputAction Object Reference" :default "/Game/Inputs/IA_Sauter.IA_Sauter"))
  ;[1 1 1] Sauter
  (:`Triggered`
    (`self.Jump`))
  (:`Completed`
    (`self.StopJumping`)))

(event `EnhancedInput|/Game/Inputs/IA_RegarderHauEtBas`
  (params (ActionValue :type "Float (double-precision)") (ElapsedSeconds :type "Float (double-precision)") (TriggeredSeconds :type "Float (double-precision)") (InputAction :type "InputAction Object Reference" :default "/Game/Inputs/IA_RegarderHauEtBas.IA_RegarderHauEtBas"))
  ;[1 1 1] Regarder Haut / Bas
  (:`Triggered`
    (`self.AddControllerPitchInput` ActionValue)))

(event `EnhancedInput|/Game/Inputs/IA_RegardeGaucheDroite`
  (params (ActionValue :type "Float (double-precision)") (ElapsedSeconds :type "Float (double-precision)") (TriggeredSeconds :type "Float (double-precision)") (InputAction :type "InputAction Object Reference" :default "/Game/Inputs/IA_RegardeGaucheDroite.IA_RegardeGaucheDroite"))
  ;[1 1 1] Regarder Gauche / Droite
  (:`Triggered`
    (`self.AddControllerYawInput` ActionValue)))

(event `EnhancedInput|/Game/Inputs/IA_LancerCubeEau`
  (params (ActionValue :type Boolean) (ElapsedSeconds :type "Float (double-precision)") (TriggeredSeconds :type "Float (double-precision)") (InputAction :type "InputAction Object Reference" :default "/Game/Inputs/IA_LancerCubeEau.IA_LancerCubeEau"))
  ;[1 1 1] Spawn du cube d'eau
  (:`Triggered`
    (`|SpawnActorFromClass` "/Game/BP_CubeEau.BP_CubeEau_C" (`KismetMathLibrary.MakeTransform` (+ (`self.K2_GetActorLocation`) (`KismetMathLibrary.GreaterGreater_VectorRotator` (`self.V_Offset`) (`self.K2_GetActorRotation`)))) "Undefined" "MultiplyWithRoot" null null)
    (`KismetSystemLibrary.PrintString` "Une cube d'eau a été crée.")))

(fn `UserConstructionScript`)